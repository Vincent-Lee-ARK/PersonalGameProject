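; BP_Enemy is an enemy Blueprint with skeletal damage and alive-check logic that reports through debug prints.
; BeginPlay prints a taunt, and the TakeDamage event prints a red scream with Health minus the damage, without storing the result.
; It then passes the unchanged Health to CheckIfAlive, which tests for above zero, but the branch does nothing.
; AliveCheckPure is an unused stub returning false.
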(event `TakeDamage`
  (params (By :type "Float (double-precision)" :default 0.2))
  (`KismetSystemLibrary.PrintString` (`KismetStringLibrary.Concat_StrStr` "AAAAH" (`KismetStringLibrary.Conv_DoubleToString` (- (`self.Health`) By))) true true (struct :`R` 1.0 :`G` 0.054336 :`A` 1.0))
  (`self.CheckIfAlive` (`self.Health`))
  (if true
    _))

(event `self.ReceiveBeginPlay`
  (`KismetSystemLibrary.PrintString` "Time to die!"))

(fn `AliveCheckPure`
  (params (Health :type "Float (double-precision)"))
  (returns (NewParam1 :type Boolean))
  (return false))

(fn `CheckIfAlive`
  (params (Health :type "Float (double-precision)"))
  (returns (Alive :type Boolean))
  (return (> Health 0.0)))

(fn `UserConstructionScript`)